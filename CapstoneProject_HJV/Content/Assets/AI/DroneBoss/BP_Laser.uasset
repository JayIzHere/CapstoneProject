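; Laser beam actor in the drone boss assets that damages the player character it hits.
; Each tick it line-traces along its forward vector, sets the beam particle's end and shows an impact effect at blocking hits.
; A hit clamps the beam length to that point and applies small per-frame damage to the player.
; The length then grows by a frame-based step (delta seconds added, not multiplied) while below its cap.
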(event EventTick
  (params (DeltaSeconds :type Float%20%28single-precision%29))
  (bind _returnvalue (Transformation|GetActorLocation))
  (bind _impacty (Variables|Default|GetImpacty))
  (Utilities|FlowControl|Sequence
    (:then_0
      (Variables|Default|SetTraceEnd (+ _returnvalue (* (Transformation|GetActorForwardVector) (Variables|Default|GetDistance))))
      (bind _outhit (Collision|LineTraceByChannel _returnvalue (+ _returnvalue (* (Transformation|GetActorForwardVector) (Variables|Default|GetDistance))) "TraceTypeQuery1" false 0 "None"))
      (Variables|Default|SetHasHit (.bblockinghit _outhit))
      (Effects|Components|ParticleSystem|SetVectorParameter (Variables|Default|GetLaser) "LaserEnd" (select (.bblockinghit _outhit) (.location _outhit) (Variables|Default|GetTraceEnd)))
      (Rendering|SetVisibility _impacty (Variables|Default|GetHasHit) false)
      (Transformation|SetWorldLocation _impacty (.location _outhit) false false)
      (if (Variables|Default|GetHasHit)
        (Variables|Default|SetDistance (Math|Vector|VectorLength (- (.location _outhit) (Transformation|GetActorLocation))))
        (bind _asplayer_character (Utilities|Casting|CastToPlayerCharacter (.hitactor _outhit)))
        (Default|TakeDamage _asplayer_character 0.15)))
    (:then_1
      (if (< (Variables|Default|GetDistance) 5e+03)
        (Variables|Default|SetDistance (+ (Variables|Default|GetDistance) (+ DeltaSeconds 2e+03)))))))

(fn ConstructionScript)