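; Grindable rail actor that builds spline mesh segments along its spline in the construction script and always reports that it can be ground.
; GetGrindSpline gives the caller the spline, start distance, offset and travel direction.
; The start is found by brute-force sampling the spline at fixed steps for the point nearest the hit.
; Direction points away from the character's side, comparing points either side of the start; CharacterSpeed is unused.
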(event EventBeginPlay
  (Rendering|SetCastShadow (Variables|Default|GetSpline) false))

(event Collision|EventActorBeginOverlap
  (params (OtherActor :type Actor%20Object%20Reference)))

(event EventTick
  (params (DeltaSeconds :type Float%20%28single-precision%29)))

(fn ConstructionScript
  (bind _spline (Variables|Default|GetSpline))
  (for _index (range 0 (Spline|GetNumberOfSplinePoints _spline))
    (bind _returnvalue (AddComponent|AddSplineMeshComponent false))
    (SplineMesh|SetStartandEnd _returnvalue (.Location (Spline|GetLocationandTangentatSplinePoint _spline _index "Local")) (.Tangent (Spline|GetLocationandTangentatSplinePoint _spline _index "Local")) (.Location (Spline|GetLocationandTangentatSplinePoint _spline (+ _index 1) "Local")) (.Tangent (Spline|GetLocationandTangentatSplinePoint _spline (+ _index 1) "Local")) true :!class /Script/Engine.SplineMeshComponent)))

(fn GetClosestDistanceAlongSpline
  (params (location :type Vector))
  (if (< (Math|Vector|Distance(Vector) location (Spline|GetLocationatDistanceAlongSpline (Variables|Default|GetSpline) (LocalVariables|Getdistance) "World")) (LocalVariables|GetminDistance)) :!label _label
    (LocalVariables|SetminDistance (Math|Vector|Distance(Vector) location (Spline|GetLocationatDistanceAlongSpline (Variables|Default|GetSpline) (LocalVariables|Getdistance) "World")))
    (LocalVariables|SetclosestDistance (LocalVariables|Getdistance)))
  (LocalVariables|Setdistance (+ (LocalVariables|Getdistance) 1e+01))
  (if (< (LocalVariables|Getdistance) (Spline|GetSplineLength (Variables|Default|GetSpline)))
    (goto _label)
    (else
      (return (LocalVariables|GetclosestDistance)))))

(fn CanGrind?
  (return true))

(fn GetGrindSpline
  (params (hit%20location :type Vector :default "0, 0, 0") (character%20location :type Vector :default "0, 0, 0") (character%20speed :type Float%20%28single-precision%29))
  (bind _spline (Variables|Default|GetSpline))
  (bind _returnvalue (Spline|GetSplineLength _spline))
  (bind _splinedistance (CallFunction|GetClosestDistanceAlongSpline hit%20location))
  (return (Variables|Default|GetSpline) _splinedistance (Math|Float|SelectFloat 1.0 -1.0 (> (Math|Vector|Distance(Vector) (Spline|GetLocationatDistanceAlongSpline _spline (Math|Float|Clamp(Float) (+ _splinedistance 2e+01) 0.0 _returnvalue) "World") character%20location) (Math|Vector|Distance(Vector) (Spline|GetLocationatDistanceAlongSpline _spline (Math|Float|Clamp(Float) (+ _splinedistance -2e+01) 0.0 _returnvalue) "World") character%20location))) (Variables|Default|GetOffset)))